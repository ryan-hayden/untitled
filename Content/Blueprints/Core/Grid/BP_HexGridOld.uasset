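; Hex grid actor that builds procedural terrain from static mesh tiles in its construction script, staggering alternate columns by an offset.
; Two FastNoise layers are sampled at each tile's location, then multiplied together and by a strength value.
; Positive results stretch the tile vertically, while others lower it through a clamp whose min and max are reversed.
; Tile height feeds the material's Elevation parameter; the HexTiles array append is never executed.
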(fn `UserConstructionScript`
  (bind _lvl_2_noise_scale (`self.Lvl 2 Noise Scale`))
  (bind _lvl_1_noise_scale (`self.Lvl 1 Noise Scale`))
  (bind _mesh (`self.Mesh`))
  (bind _mesh_2 (`self.Mesh`))
  (bind (_returnvalue_x _returnvalue_y) (`KismetMathLibrary.BreakVector` (`SceneComponent.K2_GetComponentLocation` _mesh_2)))
  ;[1 1 1] Construct Noise Level 1
  (bind _returnvalue (`|GenericCreateObject` "/Script/FastNoiseGenerator.FastNoiseWrapper"))
  (bind _output_get (set `self.FastNoiseLvl1` _returnvalue))
  (`FastNoiseWrapper.SetupFastNoise` _output_get (`self.Lvl 1 Noise Type`) (`self.Lvl 1 Seed`) (`self.Lvl 1 Frequency`) (`self.Lvl 1 Interp`) (`self.Lvl 1 Fractaltype`) (`self.Lvl 1 Octaves`) (`self.Lvl 1 Lacunarity`) (`self.Lvl 1 Gain`) (`self.Lvl 1 Cellular Jitter`) (`self.Lvl 1 Cellular Distance Function`) (`self.Lvl 1 Cellular Return Type`))
  ;[1 1 1] Construct Noise Level 2
  (bind _returnvalue_2 (`|GenericCreateObject` "/Script/FastNoiseGenerator.FastNoiseWrapper"))
  (bind _output_get_2 (set `self.FastNoiseLvl2` _returnvalue_2))
  (`FastNoiseWrapper.SetupFastNoise` _output_get_2 (`self.Lvl 2 Noise Type`) (`self.Lvl 2 Seed`) (`self.Lvl 2 Frequency`) (`self.Lvl 2 Interp`) (`self.Lvl 2 Fractaltype`) (`self.Lvl 2 Octaves`) (`self.Lvl 2 Lacunarity`) (`self.Lvl 2 Gain`) (`self.Lvl 2 Cellular Jitter`) (`self.Lvl 2 Cellular Distance Function`) (`self.Lvl 2 Cellular Return Type`))
  ;[1 1 1] Generate X/Y values
  (for _index (range 1 (+ (`self.GridX`) 1))
    (for _index_2 (range 1 (+ (`self.Grid Y`) 1))
      (bind _returnvalue_3 (* _index (`self.SpacingX`)))
      (bind _returnvalue_4 (* _index_2 (`self.SpacingY`)))
      (bind _returnvalue_5 (`AddComponent|NODE_AddStaticMeshComponent-1` :`RelativeTransform` (`KismetMathLibrary.MakeTransform` (`KismetMathLibrary.SelectVector` (`KismetMathLibrary.MakeVector` _returnvalue_3 _returnvalue_4) (`KismetMathLibrary.MakeVector` _returnvalue_3 (+ (`self.Offset`) _returnvalue_4)) (== (mod _index 2) 0)))))
      (set `self.Mesh` _returnvalue_5)
      (set `self.Coordinates` (`KismetMathLibrary.MakeVector2D` (`KismetMathLibrary.Conv_IntToDouble` _index) (`KismetMathLibrary.Conv_IntToDouble` _index_2)))
      (bind _returnvalue_6 (`SceneComponent.K2_GetComponentToWorld` _returnvalue_5))
      (bind _returnvalue_7 (* (* (`FastNoiseWrapper.GetNoise2D` (`self.FastNoiseLvl1`) (* (.x (.location _returnvalue_6)) _lvl_1_noise_scale) (* (.y (.location _returnvalue_6)) _lvl_1_noise_scale)) (`FastNoiseWrapper.GetNoise2D` (`self.FastNoiseLvl2`) (* (.x (.location _returnvalue_6)) _lvl_2_noise_scale) (* (.y (.location _returnvalue_6)) _lvl_2_noise_scale))) (`self.Strength`)))
      (if (<= _returnvalue_7 0.0)
        (bind _returnvalue_8 (`KismetMathLibrary.FClamp` _returnvalue_7 -0.1 -10.0))
        (set `self.Tile Height` (* _returnvalue_8 10.0))
        (`SceneComponent.K2_SetRelativeLocation` _mesh_2 (`KismetMathLibrary.MakeVector` _returnvalue_x _returnvalue_y _returnvalue_8) false false)
        (else
          (bind _output_get_3 (set `self.Tile Height` (* (`KismetMathLibrary.FClamp` _returnvalue_7 0.1 10.0) 10.0)))
          (`SceneComponent.SetWorldScale3D` _mesh (`KismetMathLibrary.MakeVector` 1.0 1.0 _output_get_3))))
      (`MeshComponent.SetScalarParameterValueOnMaterials` _mesh "Elevation" (`self.Tile Height`)))))