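; BP_GridVisual renders a tile grid through two BP_GridMeshInst child actors: an offset flat-mesh layer for walkable tiles and a type-colored "world" mesh layer.
; Tile updates regenerate the Grid's noise and tile types, then re-add that tile's instances.
; World tiles are stretched in Z relative to the lowest tracked height, forming terrain columns.
; SetIsWorld swaps visibility between the world layer and actors tagged "World".
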(event `self.ReceiveBeginPlay`
  (`self.SetActorTickEnabled` false))

(fn `DestroyGridVisual`
  (`|ExecutionSequence`
    (:`then_0`
      (`/Engine/EditorBlueprintResources/StandardMacros.IsValid` (`self.Grid Mesh Inst`)
        (:`Is Valid`
          (`/Game/Blueprints/Core/Grid/Utilities/BP_GridMeshInst.ClearInstances` (`self.Grid Mesh Inst`))
          (`self.SetGridLowestZ` 999999.0))))
    (:`then_1`
      (`/Engine/EditorBlueprintResources/StandardMacros.IsValid` (`self.GridMeshInstWorld`)
        (:`Is Valid`
          (`/Game/Blueprints/Core/Grid/Utilities/BP_GridMeshInst.ClearInstances` (`self.GridMeshInstWorld`))
          (`self.SetGridLowestZ` 999999.0))))))

(fn `InitializeGridVisual`
  (params (Grid :type "/Game/Blueprints/Core/Grid/BP_HexGrid Object Reference"))
  (bind (_meshsize _mesh _meshmaterial) (break `/Game/Blueprints/Core/Grid/S_GridShapeData` (`/Game/Blueprints/Core/Grid/BP_HexGrid.GetCurrentShapeData` (`self.Grid`))))
  (bind (_meshsize_2 _mesh_2 _meshmaterial_2 _flatmesh _watermaterial _normalmaterial) (break `/Game/Blueprints/Core/Grid/S_GridShapeData` (`/Game/Blueprints/Core/Grid/BP_HexGrid.GetCurrentShapeData` (`self.Grid`))))
  (set `self.Grid` Grid)
  (bind _output_get (set `self.Grid Mesh Inst` (cast `/Game/Blueprints/Core/Grid/Utilities/BP_GridMeshInst` (`ChildActorComponent.ChildActor` (`self.ChildActor_GridMeshInst`)) :!pure true)))
  (set `self.GridMeshInstWorld` (cast `/Game/Blueprints/Core/Grid/Utilities/BP_GridMeshInst` (`ChildActorComponent.ChildActor` (`self.ChildActor_GridMeshInstWorld`)) :!pure true))
  (`/Game/Blueprints/Core/Grid/Utilities/BP_GridMeshInst.InitializeGridMeshInst` _output_get _flatmesh _watermaterial _normalmaterial false "QueryOnly" "NewEnumerator0")
  (`/Game/Blueprints/Core/Grid/Utilities/BP_GridMeshInst.InitializeGridMeshInst` (`self.GridMeshInstWorld`) _mesh _meshmaterial _meshmaterial true "QueryOnly" "NewEnumerator0")
  ;[1 1 1] Center Grid In World
  (`self.K2_SetActorLocation` (0.0 0.0 0.0))
  (`self.SetOffsetFromGround` (`self.OffsetFromGround`))
  (`self.SetGridLowestZ` 999999.0))

(fn `SetGridLowestZ`
  (params (GridLowestZ :type "Float (double-precision)"))
  (set `self.Z` GridLowestZ))

(fn `SetIsWorld`
  (params (IsWorldVisible :type Boolean))
  (set `self.Is World Visible` IsWorldVisible)
  (`SceneComponent.SetHiddenInGame` (`self.ChildActor_GridMeshInstWorld`) (not (`self.Is World Visible`)) false)
  (bind _outactors (`GameplayStatics.GetAllActorsWithTag` "World"))
  (for _array_element _outactors
    (`self.SetActorHiddenInGame` _array_element (`self.Is World Visible`))))

(fn `SetOffsetFromGround`
  (params (Offset :type "Float (double-precision)"))
  (bind _output_get (set `self.OffsetFromGround` Offset))
  (`SceneComponent.K2_SetRelativeLocation` (`self.ChildActor_GridMeshInst`) (`KismetMathLibrary.MakeVector` 0.0 0.0 _output_get) false false))

(fn `UpdateTileVisual`
  (params (Data :type "/Game/Blueprints/Core/Grid/Utilities/S_TileData Structure"))
  (bind (_data_index _data_type _data_transform _data_states) (break `/Game/Blueprints/Core/Grid/Utilities/S_TileData` (`local.Data`)))
  (bind _grid (`self.Grid`))
  (bind (_data_index_2 _data_type_2) (break `/Game/Blueprints/Core/Grid/Utilities/S_TileData` (`local.Data`)))
  (`/Game/Blueprints/Core/Grid/BP_HexGrid.GenerateNoise` _grid)
  (`/Game/Blueprints/Core/Grid/BP_HexGrid.GenerateTileTypeFromNoise` :`self` _grid)
  (`|ExecutionSequence`
    (:`then_0`
      (`/Game/Blueprints/Core/Grid/Utilities/BP_GridMeshInst.RemoveInstance` (`self.Grid Mesh Inst`) _data_index_2)
      (if (`/Game/Blueprints/Core/Utilities/BFL_TileData.IsTileTypeWalkable` _data_type_2)
        (`/Game/Blueprints/Core/Grid/Utilities/BP_GridMeshInst.AddInstance` (`self.Grid Mesh Inst`) _data_transform _data_index _data_states _data_type)))
    (:`then_1`
      (`self.UpdateTileVisualWorld` Data))))

(fn `UpdateTileVisualWorld`
  (params (Data :type "/Game/Blueprints/Core/Grid/Utilities/S_TileData Structure"))
  (bind (_data_index _data_type _data_transform) (break `/Game/Blueprints/Core/Grid/Utilities/S_TileData` (`local.Data`)))
  (bind (_data_index_2 _data_type_2 _data_transform_2 _data_states) (break `/Game/Blueprints/Core/Grid/Utilities/S_TileData` (`local.Data`)))
  (bind (_data_index_3 _data_type_3 _data_transform_3) (break `/Game/Blueprints/Core/Grid/Utilities/S_TileData` (`local.Data`)))
  (bind (_data_index_4 _data_type_4) (break `/Game/Blueprints/Core/Grid/Utilities/S_TileData` (`local.Data`)))
  (bind _z (.z (`.MeshSize_2_CDFA6A6D462F7184638BBD8439C247DD` (break `/Game/Blueprints/Core/Grid/S_GridShapeData` (`/Game/Blueprints/Core/Grid/BP_HexGrid.GetCurrentShapeData` (`self.Grid`))))))
  (`|ExecutionSequence`
    (:`then_0`
      (if (< (.z (.location _data_transform_3)) (`self.Z`))
        (`self.SetGridLowestZ` (.z (.location _data_transform_3)))))
    (:`then_1`
      (`/Game/Blueprints/Core/Grid/Utilities/BP_GridMeshInst.RemoveInstance` (`self.GridMeshInstWorld`) _data_index_4)
      (if (`|EnumInequality` _data_type_4 "NewEnumerator0")
        (`/Game/Blueprints/Core/Grid/Utilities/BP_GridMeshInst.AddInstance` (`self.GridMeshInstWorld`) (`KismetMathLibrary.MakeTransform` (.location _data_transform_2) (.rotation _data_transform_2) (`KismetMathLibrary.MakeVector` (.x (.scale _data_transform_2)) (.y (.scale _data_transform_2)) (/ (+ (- (.z (.location _data_transform)) (`self.Z`)) _z) _z))) _data_index_2 _data_states _data_type_2)))))

(fn `UserConstructionScript`)