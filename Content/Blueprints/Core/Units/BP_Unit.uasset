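; Base grid-tactics unit actor that loads its mesh, animation and stats from its unit type and shows hover, selection and team color.
; A timeline walks it tile by tile along a path, broadcasting movement events.
; Clamped setters manage HP, movement and action points; abilities check and spend AP.
; Hits change HP immediately but defer health bar, damage number and hit/death animation until the ability animation reaches the unit's tile.
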(event `self.ReceiveBeginPlay`
  (`self.SetAnimationState` "NewEnumerator0")
  (bind _output_get (set `self.Health Bar` (cast `/Game/Blueprints/Core/Units/Widgets/W_HealthBar` (`WidgetComponent.GetUserWidgetObject` (`self.Widget`)) :!pure true)))
  (`/Game/Blueprints/Core/Units/Widgets/W_HealthBar.Event_SetUnit` _output_get self))

(event `Event_FollowPath`
  (params (Path :type "Array of IntPoint Structure"))
  (if (> (`KismetArrayLibrary.Array_Length` Path) 0)
    (set `self.CurrentPath` Path)
    (`self.OnUnitStartedWalking` self)
    (`self.Event_ContinueToFollowPath`)))

(event `Event_ContinueToFollowPath`
  (bind (_previoustransform_location _previoustransform_rotation) (`KismetMathLibrary.BreakTransform` (`self.PreviousTransform`)))
  (bind (_nexttransform_location _nexttransform_rotation) (`KismetMathLibrary.BreakTransform` (`self.NextTransform`)))
  (bind _previoustransform_location_2 (`KismetMathLibrary.BreakTransform` (`self.PreviousTransform`)))
  (bind _timeline_unitmovement (`self.Timeline_UnitMovement`))
  (bind (_index _type _transform) (break `/Game/Blueprints/Core/Grid/Utilities/S_TileData` (`BlueprintMapLibrary.Map_Find` (`/Game/Blueprints/Core/Grid/BP_HexGrid.GridTiles` (`self.Grid`)) (`|GetArrayItem` (`self.CurrentPath`)))))
  (if (> (`KismetArrayLibrary.Array_Length` (`self.CurrentPath`)) 0)
    (`self.SetAnimationState` "NewEnumerator1")
    (set `self.PreviousTransform` (`self.GetTransform`))
    (set `self.NextTransform` (`KismetMathLibrary.MakeTransform` (.location _transform) (`KismetMathLibrary.FindLookAtRotation` _previoustransform_location_2 (.location _transform))))
    (`TimelineComponent.SetPlayRate` _timeline_unitmovement (/ (`TimelineComponent.GetTimelineLength` _timeline_unitmovement) (`self.MoveDurationPerTile`)))
    (bind (_direction _locationalpha _rotationalpha) (`Timeline|Timeline_UnitMovement` :!via `PlayFromStart`)
      (:`Update`
        (`self.K2_SetActorLocationAndRotation` (`KismetMathLibrary.VLerp` _previoustransform_location _nexttransform_location _locationalpha) (`KismetMathLibrary.RLerp` _previoustransform_rotation _nexttransform_rotation _rotationalpha true)))
      (:`Finished`
        (`self.OnUnitReachNewTile` (`|GetArrayItem` (`self.CurrentPath`)) self)
        (`KismetArrayLibrary.Array_Remove` (`self.CurrentPath`))
        (`self.Event_ContinueToFollowPath`)))
    (else
      (`self.SetAnimationState` "NewEnumerator0")
      (`self.OnUnitFinishedWalking` self))))

(event `Event_DestroyUnitAfterDelayOnDeath`)

(fn `CanUseAbility`
  (params (`Ability Data` :type "/Game/Blueprints/Core/Combat/Abilities/Utilities/S_AbilityData Structure"))
  (returns (`Can Use Ability` :type Boolean))
  (if (`KismetArrayLibrary.Array_Contains` (`.Abilities_13_6A88051846051275BA6C9DB661243998` (break `/Game/Blueprints/Core/Units/Utilities/S_UnitData_Stats` (`.Stats_8_259033F3475D35C48E71B89EEDD5F0C2` (break `/Game/Blueprints/Core/Units/Utilities/S_UnitData` (`self.UnitData`))))) (`.Ability_3_DE8D6A8C4EBE0AAB1E4F08AC8D26E020` (break `/Game/Blueprints/Core/Combat/Abilities/Utilities/S_AbilityData` (`local.Ability Data`))))
    (if (>= (`.CurrentActionPoints_37_FADB54834243D48468B0ACBFA97BE455` (break `/Game/Blueprints/Core/Units/Utilities/S_UnitData_Stats` (`.Stats_8_259033F3475D35C48E71B89EEDD5F0C2` (break `/Game/Blueprints/Core/Units/Utilities/S_UnitData` (`self.UnitData`))))) (`.Cost_AP_2_39BED71C4F1C823D2946289C67598245` (break `/Game/Blueprints/Core/Combat/Abilities/Utilities/S_AbilityData_Requirements` (`.Requirements_20_1278378A45348A5A405DCA85DD43A20F` (break `/Game/Blueprints/Core/Combat/Abilities/Utilities/S_AbilityData` (`local.Ability Data`))))))
      (return true)
      (else
        (return false)))
    (else
      (return false))))

(fn `Combat Ended`
  (`KismetSystemLibrary.PrintString` "fuck"))

(fn `CombatStarted`
  (`KismetSystemLibrary.PrintString` "shit")
  (`self.ResetMovementPoints`)
  (`self.ResetActionPoints`))

(fn `GetAnimationState`
  (returns (State :type "/Game/Assets/Units/E_UnitAnimationState Enum"))
  (bind _state (message `/Game/Assets/Units/BPI_UnitAnimation.GetUnitAnimationState` (`SkeletalMeshComponent.GetAnimInstance` (`self.SkeletalMesh`))))
  (return _state))

(fn `IsAlive`
  (returns (IsAlive :type Boolean))
  (if (> (`.HPCurrent_18_71789C4E47F0543A884B65A3A23A9D64` (break `/Game/Blueprints/Core/Units/Utilities/S_UnitData_Stats` (`.Stats_8_259033F3475D35C48E71B89EEDD5F0C2` (break `/Game/Blueprints/Core/Units/Utilities/S_UnitData` (`self.UnitData`))))) 0.0)
    (return true)))

(fn `ModifyCurrentActionPoints`
  (params (Modifier :type Integer))
  (`self.SetCurrentActionPoints` (+ Modifier (`.CurrentActionPoints_37_FADB54834243D48468B0ACBFA97BE455` (break `/Game/Blueprints/Core/Units/Utilities/S_UnitData_Stats` (`.Stats_8_259033F3475D35C48E71B89EEDD5F0C2` (break `/Game/Blueprints/Core/Units/Utilities/S_UnitData` (`self.UnitData`))))))))

(fn `ModifyCurrentHP`
  (params (Modifier :type "Float (double-precision)"))
  (`self.SetCurrentHp` (+ Modifier (`.HPCurrent_18_71789C4E47F0543A884B65A3A23A9D64` (break `/Game/Blueprints/Core/Units/Utilities/S_UnitData_Stats` (`.Stats_8_259033F3475D35C48E71B89EEDD5F0C2` (break `/Game/Blueprints/Core/Units/Utilities/S_UnitData` (`self.UnitData`))))))))

(fn `ModifyCurrentMovementPoints`
  (params (Modifier :type Integer))
  (`self.SetCurrentMovementPoints` (+ Modifier (`.CurrentMovementPoints_33_54C2012E4EF67102CC8357A986711646` (break `/Game/Blueprints/Core/Units/Utilities/S_UnitData_Stats` (`.Stats_8_259033F3475D35C48E71B89EEDD5F0C2` (break `/Game/Blueprints/Core/Units/Utilities/S_UnitData` (`self.UnitData`))))))))

(fn `OnAbilityAnimationHitTile`
  (params (AbilityAnimation :type "/Game/Blueprints/Core/Combat/Abilities/BP_AbilityAnimation Object Reference") (`Hit Index` :type "IntPoint Structure"))
  (locals (AbilityImpactReal :type "/Game/Blueprints/Core/Combat/Abilities/Utilities/S_AbilityData_Impact_Real Structure"))
  (bind (_value _returnvalue) (`BlueprintMapLibrary.Map_Find` (`self.IncomingAbilityAnimations`) AbilityAnimation))
  (if (`KismetMathLibrary.Equal_IntPointIntPoint` (`self.Index`) `Hit Index`)
    (if _returnvalue
      (set `local.AbilityImpactReal` _value)
      (`BlueprintMapLibrary.Map_Remove` (`self.IncomingAbilityAnimations`) (`local.AbilityAnimation`))
      (if (!= (`.Modifier_Hp_4_68274EFA4A068D2AD37DA7A7990DB3FE` (break `/Game/Blueprints/Core/Combat/Abilities/Utilities/S_AbilityData_Impact_Real` (`local.AbilityImpactReal`))) 0.0)
        (`/Game/Blueprints/Core/Units/Widgets/W_HealthBar.Event_UpdateHealthBar` (`self.Health Bar`))
        (`|SpawnActorFromClass` "/Game/Blueprints/Core/Units/Widgets/BP_AnimatedNumber.BP_AnimatedNumber_C" (`KismetMathLibrary.MakeTransform` (`self.K2_GetActorLocation`)) "Undefined" "MultiplyWithRoot" null (`.Modifier_Hp_4_68274EFA4A068D2AD37DA7A7990DB3FE` (break `/Game/Blueprints/Core/Combat/Abilities/Utilities/S_AbilityData_Impact_Real` (`local.AbilityImpactReal`))) null)
        (if (< (`.Modifier_Hp_4_68274EFA4A068D2AD37DA7A7990DB3FE` (break `/Game/Blueprints/Core/Combat/Abilities/Utilities/S_AbilityData_Impact_Real` (`local.AbilityImpactReal`))) 0.0)
          (if (not (`self.IsAlive`))
            (if (`|EnumInequality` (`self.GetAnimationState`) "NewEnumerator4")
              (`self.SetAnimationState` "NewEnumerator4"))
            (else
              (`self.SetAnimationState` "NewEnumerator2"))))))))

(fn `Planning Ended`)

(fn `Planning Started`)

(fn `ResetActionPoints`
  (`self.SetCurrentActionPoints` (`.MaxActionPoints_36_B62F41E345D96756D4F18D9C52179F44` (break `/Game/Blueprints/Core/Units/Utilities/S_UnitData_Stats` (`.Stats_8_259033F3475D35C48E71B89EEDD5F0C2` (break `/Game/Blueprints/Core/Units/Utilities/S_UnitData` (`self.UnitData`)))))))

(fn `ResetMovementPoints`
  (`self.SetCurrentMovementPoints` (`.MaxMovementPoints_32_9EC431674FDDE6E5EAE61880BA02F359` (break `/Game/Blueprints/Core/Units/Utilities/S_UnitData_Stats` (`.Stats_8_259033F3475D35C48E71B89EEDD5F0C2` (break `/Game/Blueprints/Core/Units/Utilities/S_UnitData` (`self.UnitData`)))))))

(fn `SetAnimationState`
  (params (NewParam :type "/Game/Assets/Units/E_UnitAnimationState Enum" :default "NewEnumerator0"))
  (message `/Game/Assets/Units/BPI_UnitAnimation.SetUnitAnimationState` (`SkeletalMeshComponent.GetAnimInstance` (`self.SkeletalMesh`)) NewParam))

(fn `SetCurrentActionPoints`
  (params (`Action Points` :type Integer))
  (locals (Difference :type Integer))
  (bind (_validtiletypes _currentmovementpoints _maxmovementpoints _abilities _hpcurrent _hpmax _initiative _currentactionpoints _maxactionpoints) (break `/Game/Blueprints/Core/Units/Utilities/S_UnitData_Stats` (`.Stats_8_259033F3475D35C48E71B89EEDD5F0C2` (break `/Game/Blueprints/Core/Units/Utilities/S_UnitData` (`self.UnitData`)))))
  (set `local.Difference` (- `Action Points` _currentactionpoints))
  (bind _structout (setmembers `/Game/Blueprints/Core/Units/Utilities/S_UnitData_Stats` :`StructRef` (`.Stats_8_259033F3475D35C48E71B89EEDD5F0C2` (break `/Game/Blueprints/Core/Units/Utilities/S_UnitData` (`self.UnitData`))) :`CurrentAction Points` (`KismetMathLibrary.Clamp` `Action Points` 0 _maxactionpoints)))
  (setmembers `/Game/Blueprints/Core/Units/Utilities/S_UnitData` :`StructRef` (`self.UnitData`) :`Stats` _structout)
  (`self.OnUnitStatChanged` self))

(fn `SetCurrentHp`
  (params (Hp :type "Float (double-precision)"))
  (bind _structout (setmembers `/Game/Blueprints/Core/Units/Utilities/S_UnitData_Stats` :`StructRef` (`.Stats_8_259033F3475D35C48E71B89EEDD5F0C2` (break `/Game/Blueprints/Core/Units/Utilities/S_UnitData` (`self.UnitData`))) :`HP Current` (/ (`KismetMathLibrary.FFloor` (* (`KismetMathLibrary.FClamp` Hp 0.0 (`.HPMax_19_9A85F02E4CF2ADA4FD06DF9FC7EE1673` (break `/Game/Blueprints/Core/Units/Utilities/S_UnitData_Stats` (`.Stats_8_259033F3475D35C48E71B89EEDD5F0C2` (break `/Game/Blueprints/Core/Units/Utilities/S_UnitData` (`self.UnitData`)))))) 10.0)) 10)))
  (setmembers `/Game/Blueprints/Core/Units/Utilities/S_UnitData` :`StructRef` (`self.UnitData`) :`Stats` _structout)
  (`self.OnUnitStatChanged` self))

(fn `SetCurrentMovementPoints`
  (params (MovementPoints :type Integer))
  (locals (Difference :type Integer))
  (bind (_validtiletypes _currentmovementpoints _maxmovementpoints) (break `/Game/Blueprints/Core/Units/Utilities/S_UnitData_Stats` (`.Stats_8_259033F3475D35C48E71B89EEDD5F0C2` (break `/Game/Blueprints/Core/Units/Utilities/S_UnitData` (`self.UnitData`)))))
  (set `local.Difference` (- MovementPoints _currentmovementpoints))
  (bind _structout (setmembers `/Game/Blueprints/Core/Units/Utilities/S_UnitData_Stats` :`StructRef` (`.Stats_8_259033F3475D35C48E71B89EEDD5F0C2` (break `/Game/Blueprints/Core/Units/Utilities/S_UnitData` (`self.UnitData`))) :`CurrentMovement Points` (`KismetMathLibrary.Clamp` MovementPoints 0 _maxmovementpoints)))
  (setmembers `/Game/Blueprints/Core/Units/Utilities/S_UnitData` :`StructRef` (`self.UnitData`) :`Stats` _structout)
  (`self.OnUnitStatChanged` self))

(fn `SetGrid`
  (params (Grid :type "/Game/Blueprints/Core/Grid/BP_HexGrid Object Reference"))
  (bind _staticmesh_teamindex (`self.StaticMesh_TeamIndex`))
  (bind (_returnvalue_x _returnvalue_y _returnvalue_z) (`KismetMathLibrary.BreakVector` (`SceneComponent.K2_GetComponentScale` (`self.Collision_LineOfSight`))))
  (bind (_meshsize _mesh _meshmaterial _flatmesh _watermaterial _normalmaterial) (break `/Game/Blueprints/Core/Grid/S_GridShapeData` (`/Game/Blueprints/Core/Grid/BP_HexGrid.GetCurrentShapeData` (`self.Grid`))))
  (bind (_returnvalue_x_2 _returnvalue_y_2) (`KismetMathLibrary.BreakVector` (/ (`/Game/Blueprints/Core/Grid/BP_HexGrid.Grid Tile Size` (`self.Grid`)) (`.MeshSize_2_CDFA6A6D462F7184638BBD8439C247DD` (break `/Game/Blueprints/Core/Grid/S_GridShapeData` (`/Game/Blueprints/Core/Grid/BP_HexGrid.GetCurrentShapeData` (`self.Grid`)))))))
  (set `self.Grid` Grid)
  ;[1 1 1] Sets Collision for Line of Sight to match the size of the grid
  (`SceneComponent.SetWorldScale3D` (`self.Collision_LineOfSight`) (`KismetMathLibrary.MakeVector` _returnvalue_x_2 _returnvalue_y_2 _returnvalue_z))
  (`StaticMeshComponent.SetStaticMesh` _staticmesh_teamindex _flatmesh)
  (`PrimitiveComponent.SetMaterial` _staticmesh_teamindex 0 _normalmaterial)
  (`MeshComponent.SetScalarParameterValueOnMaterials` _staticmesh_teamindex "IsFilled" 1.0)
  (`SceneComponent.SetAbsolute` _staticmesh_teamindex false true true)
  (`SceneComponent.SetWorldScale3D` _staticmesh_teamindex (/ (`/Game/Blueprints/Core/Grid/BP_HexGrid.Grid Tile Size` (`self.Grid`)) _meshsize))
  (`SceneComponent.K2_SetRelativeLocation` _staticmesh_teamindex (`KismetMathLibrary.MakeVector` 0.0 0.0 (/ (`/Game/Blueprints/Core/Grid/BP_GridVisual.OffsetFromGround` (`/Game/Blueprints/Core/Grid/BP_HexGrid.Grid Visual` (`self.Grid`))) 5.0)) false false))

(fn `SetIsHovered`
  (params (Hovered :type Boolean))
  (set `self.IsHovered` Hovered)
  (`self.UpdateColorIfHoveredOrSelected`))

(fn `SetIsSelected`
  (params (Selected :type Boolean))
  (set `self.IsSelected` Selected)
  (`self.UpdateColorIfHoveredOrSelected`))

(fn `SetTeamIndex`
  (params (`Team Index` :type Integer))
  (set `self.Team Index` `Team Index`)
  (`ProgressBar.SetFillColorAndOpacity` (`/Game/Blueprints/Core/Units/Widgets/W_HealthBar.ProgressBar_Health` (`self.Health Bar`)) (`/Game/Blueprints/Core/Combat/Utilities/BFL_Combat.GetTeamColor` (`self.Team Index`)))
  (`MeshComponent.SetVectorParameterValueOnMaterials` (`self.StaticMesh_TeamIndex`) "Color" (`KismetMathLibrary.Conv_LinearColorToVector` (`/Game/Blueprints/Core/Combat/Utilities/BFL_Combat.GetTeamColor` (`self.Team Index`)))))

(fn `SetUnitData`
  (params (Data :type "/Game/Blueprints/Core/Units/Utilities/S_UnitData Structure (by ref)"))
  (bind _skeletalmesh (`self.SkeletalMesh`))
  (bind (_mesh _animationblueprint) (break `/Game/Blueprints/Core/Units/Utilities/S_UnitData_Assets` (`.Assets_5_21AA228B4B4A4B0DBACEB79490021B31` (break `/Game/Blueprints/Core/Units/Utilities/S_UnitData` Data))))
  (set `self.UnitData` Data)
  (`SkeletalMeshComponent.SetSkeletalMeshAsset` _skeletalmesh _mesh)
  (`SkeletalMeshComponent.SetAnimInstanceClass` _skeletalmesh _animationblueprint)
  (`self.UpdateColorIfHoveredOrSelected`)
  (`self.OnUnitStatChanged` self))

(fn `UnitHitByAbility`
  (params (`Ability Impact Real` :type "/Game/Blueprints/Core/Combat/Abilities/Utilities/S_AbilityData_Impact_Real Structure") (AbilityAnimation :type "/Game/Blueprints/Core/Combat/Abilities/BP_AbilityAnimation Object Reference"))
  (locals (HpModifier :type "Float (double-precision)"))
  (bind _modifier_hp (break `/Game/Blueprints/Core/Combat/Abilities/Utilities/S_AbilityData_Impact_Real` (`local.Ability Impact Real`)))
  (`BlueprintMapLibrary.Map_Add` (`self.IncomingAbilityAnimations`) AbilityAnimation `Ability Impact Real`)
  (add `/Game/Blueprints/Core/Combat/Abilities/BP_AbilityAnimation.OnAbilityAnimationHitTile` AbilityAnimation (`|CreateDelegate` :!event `OnAbilityAnimationHitTile`))
  (if (!= _modifier_hp 0.0)
    (bind _output_get (set `local.HpModifier` _modifier_hp))
    (`self.ModifyCurrentHP` _output_get)))

(fn `UnitUseAbility`
  (params (`Target Index` :type "IntPoint Structure") (AbilityData :type "/Game/Blueprints/Core/Combat/Abilities/Utilities/S_AbilityData Structure"))
  (bind (_returnvalue_x _returnvalue_y) (`KismetMathLibrary.BreakVector` (`self.K2_GetActorLocation`)))
  (`self.K2_SetActorRotation` (`KismetMathLibrary.FindLookAtRotation` (`KismetMathLibrary.MakeVector` _returnvalue_x _returnvalue_y) (`KismetMathLibrary.MakeVector` (.x (.location (`.Transform_8_1D847D9A429058A71E48E482CDEF505D` (break `/Game/Blueprints/Core/Grid/Utilities/S_TileData` (`BlueprintMapLibrary.Map_Find` (`/Game/Blueprints/Core/Grid/BP_HexGrid.GridTiles` (`self.Grid`)) `Target Index`))))) (.y (.location (`.Transform_8_1D847D9A429058A71E48E482CDEF505D` (break `/Game/Blueprints/Core/Grid/Utilities/S_TileData` (`BlueprintMapLibrary.Map_Find` (`/Game/Blueprints/Core/Grid/BP_HexGrid.GridTiles` (`self.Grid`)) `Target Index`))))))))
  (`self.SetAnimationState` "NewEnumerator3")
  (`self.ModifyCurrentActionPoints` (- 0 (`.Cost_AP_2_39BED71C4F1C823D2946289C67598245` (break `/Game/Blueprints/Core/Combat/Abilities/Utilities/S_AbilityData_Requirements` (`.Requirements_20_1278378A45348A5A405DCA85DD43A20F` (break `/Game/Blueprints/Core/Combat/Abilities/Utilities/S_AbilityData` (`local.AbilityData`))))))))

(fn `UpdateColorIfHoveredOrSelected`
  (`MeshComponent.SetVectorParameterValueOnMaterials` (`self.SkeletalMesh`) "ColorMultiply" (`KismetMathLibrary.Conv_LinearColorToVector` (* (`KismetMathLibrary.SelectFloat` 2.5 1.0 (`self.IsSelected`)) (* (`KismetMathLibrary.SelectFloat` 2.5 1.0 (`self.IsHovered`)) (`KismetMathLibrary.SelectColor` (struct :`G` 0.665732 :`B` 1.0 :`A` 1.0) (struct :`R` 0.973152 :`G` 0.926343 :`B` 1.0 :`A` 1.0) (`self.IsSelected`)))))))

(fn `UserConstructionScript`
  (bind _unit_data (`/Game/Blueprints/Core/Units/Utilities/BFL_Units.GetDefaultUnitDataFromUnitType` (`self.Unit Type`)))
  (`self.SetUnitData` _unit_data))