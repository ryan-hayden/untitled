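; BP_Controller is the player controller, which shows the mouse cursor on play and toggles a pause menu.
; The IA_Pause input flips an IsPaused flag, creating W_PauseMenu on pause and removing it on resume.
; Pausing removes top-level W_DebugMenu widgets, with SetGamePaused(true) called inside that removal loop, so it only runs when one exists.
; Resuming unpauses the game and adds a fresh W_DebugMenu to the viewport.
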(event `self.ReceiveBeginPlay`
  (set `self.bShowMouseCursor` true))

(event `EnhancedInput|/Game/Input/Mappings/IA_Pause`
  (params (ActionValue :type Boolean) (ElapsedSeconds :type "Float (double-precision)") (TriggeredSeconds :type "Float (double-precision)") (InputAction :type "InputAction Object Reference" :default "/Game/Input/Mappings/IA_Pause.IA_Pause"))
  ;[1 1 1] Toggle Pause
  (:`Triggered`
    (if (`self.IsPaused`)
      (set `self.IsPaused` false)
      (`GameplayStatics.SetGamePaused` false)
      (`Widget.RemoveFromParent` (stale _returnvalue_2))
      (bind _returnvalue (`|CreateWidget` "/Game/Blueprints/DebugMenu/W_DebugMenu.W_DebugMenu_C"))
      (`UserWidget.AddToViewport` _returnvalue 0)
      (else
        (set `self.IsPaused` true)
        (bind _returnvalue_2 (`|CreateWidget` "/Game/Blueprints/Core/UI/Widgets/W_PauseMenu.W_PauseMenu_C"))
        (bind _output_get (set `self.PauseMenu` _returnvalue_2))
        (`UserWidget.AddToViewport` _output_get 0)
        (bind _foundwidgets (`WidgetBlueprintLibrary.GetAllWidgetsOfClass` "/Game/Blueprints/DebugMenu/W_DebugMenu.W_DebugMenu_C"))
        (for _array_element _foundwidgets
          (`Widget.RemoveFromParent` _array_element)
          (`GameplayStatics.SetGamePaused` true))))))

(fn `UserConstructionScript`)