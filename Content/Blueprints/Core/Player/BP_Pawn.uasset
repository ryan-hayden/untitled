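; Player camera pawn with a spring arm that pans, rotates and zooms through Enhanced Input.
; Input events only update target location, rotation and zoom distance, which Tick interpolates toward for smoothed motion.
; Zoom is clamped; IA_ZoomIn and IA_ZoomOut use hardcoded steps and limits rather than the zoom variables used by IA_Zoom.
; CheckMouse holds screen-edge scrolling logic but is never executed.
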(event `self.ReceiveBeginPlay`
  (bind _returnvalue (pcsubsystem `EnhancedInputLocalPlayerSubsystem` (cast `PlayerController` (`self.GetOwner`) :!pure true)))
  ;[1 1 1] Set Input Mappings to Enhanced Input Subsystem
  (`/Engine/EditorBlueprintResources/StandardMacros.IsValid` _returnvalue
    (:`Is Valid`
      (`EnhancedInputSubsystemInterface.AddMappingContext` _returnvalue "/Game/Input/IAC_DefaultInput.IAC_DefaultInput" 0 (struct))
      ;[1 1 1] Set Starting Zoom
      (set `self.ZoomDistance` (`SpringArmComponent.TargetArmLength` (`self.SpringArm`))))))

(event `self.ReceiveTick`
  (params (DeltaSeconds :type "Float (single-precision)"))
  (bind _springarm (`self.SpringArm`))
  ;[1 1 1] Set Zoom Length
  (set `SpringArmComponent.TargetArmLength` (`KismetMathLibrary.FInterpTo` (`SpringArmComponent.TargetArmLength` _springarm) (`self.ZoomDistance`) DeltaSeconds (`self.Zoom Smoothness`)) _springarm)
  ;[1 1 1] Move Camera
  (`self.K2_SetActorLocation` (`KismetMathLibrary.VInterpTo` (`self.K2_GetActorLocation`) (`self.Location`) DeltaSeconds (`self.LocationSmoothness`)))
  ;[1 1 1] Set Rotation
  (`self.K2_SetActorRotation` (`KismetMathLibrary.RInterpTo` (`self.K2_GetActorRotation`) (`self.Rotation`) DeltaSeconds (`self.RotationSmoothness`))))

(event `EnhancedInput|/Game/Input/Mappings/IA_Zoom`
  (params (ActionValue :type "Float (double-precision)") (ElapsedSeconds :type "Float (double-precision)") (TriggeredSeconds :type "Float (double-precision)") (InputAction :type "InputAction Object Reference" :default "/Game/Input/Mappings/IA_Zoom.IA_Zoom"))
  ;[1 1 1] Zoom Function
  (:`Triggered`
    (set `self.ZoomDistance` (`KismetMathLibrary.FClamp` (+ (* ActionValue (`self.Zoom Speed`)) (`self.ZoomDistance`)) (`self.ZoomMin`) (`self.ZoomMax`)))))

(event `EnhancedInput|/Game/Input/Mappings/IA_ZoomIn`
  (params (ActionValue :type "Float (double-precision)") (ElapsedSeconds :type "Float (double-precision)") (TriggeredSeconds :type "Float (double-precision)") (InputAction :type "InputAction Object Reference" :default "/Game/Input/Mappings/IA_ZoomIn.IA_ZoomIn"))
  ;[1 1 1] Zoom Function
  (:`Triggered`
    (set `self.ZoomDistance` (`KismetMathLibrary.FClamp` (+ (* ActionValue -25.0) (`self.ZoomDistance`)) 300.0 7000.0))))

(event `EnhancedInput|/Game/Input/Mappings/IA_ZoomOut`
  (params (ActionValue :type "Float (double-precision)") (ElapsedSeconds :type "Float (double-precision)") (TriggeredSeconds :type "Float (double-precision)") (InputAction :type "InputAction Object Reference" :default "/Game/Input/Mappings/IA_ZoomOut.IA_ZoomOut"))
  ;[1 1 1] Zoom Function
  (:`Triggered`
    (set `self.ZoomDistance` (`KismetMathLibrary.FClamp` (+ (* ActionValue 25.0) (`self.ZoomDistance`)) 300.0 7000.0))))

(event `EnhancedInput|/Game/Input/Mappings/IA_CameraMove`
  (params (ActionValue :type "Vector2D Structure") (ElapsedSeconds :type "Float (double-precision)") (TriggeredSeconds :type "Float (double-precision)") (InputAction :type "InputAction Object Reference" :default "/Game/Input/Mappings/IA_CameraMove.IA_CameraMove"))
  (bind (_returnvalue_x _returnvalue_y) (`KismetMathLibrary.BreakVector2D` (`KismetMathLibrary.Normal2D` ActionValue)))
  ;[1 1 1] Move Camera
  (:`Triggered`
    (set `self.Location` (+ (* (`self.GetActorForwardVector`) (* _returnvalue_x (`self.LocationSpeed`))) (`self.Location`) (* (`self.GetActorRightVector`) (* _returnvalue_y (`self.LocationSpeed`)))))))

(event `EnhancedInput|/Game/Input/Mappings/IA_CameraRotate`
  (params (ActionValue :type "Float (double-precision)") (ElapsedSeconds :type "Float (double-precision)") (TriggeredSeconds :type "Float (double-precision)") (InputAction :type "InputAction Object Reference" :default "/Game/Input/Mappings/IA_CameraRotate.IA_CameraRotate"))
  ;[1 1 1] Rotate Camera
  (:`Triggered`
    (set `self.Rotation` (`KismetMathLibrary.ComposeRotators` (`self.Rotation`) (`KismetMathLibrary.MakeRotator` 0.0 0.0 (* ActionValue (`self.RotationSpeed`)))))))

(fn `CheckMouse`
  (bind (_returnvalue_x _returnvalue_y) (`KismetMathLibrary.BreakVector2D` (`WidgetLayoutLibrary.GetViewportSize`)))
  (bind (_returnvalue_x_2 _returnvalue_y_2) (`KismetMathLibrary.BreakVector2D` (`WidgetLayoutLibrary.GetViewportSize`)))
  (bind _returnvalue_x_3 (`KismetMathLibrary.BreakVector2D` (`WidgetLayoutLibrary.GetViewportSize`)))
  (bind _returnvalue_x_4 (`KismetMathLibrary.BreakVector2D` (`WidgetLayoutLibrary.GetViewportSize`)))
  (bind _returnvalue (`WidgetLayoutLibrary.GetMousePositionOnViewport`))
  (set `self.Mouse X` (`KismetMathLibrary.BreakVector2D` _returnvalue))
  (set `self.Mouse Y` (`.Y` (`KismetMathLibrary.BreakVector2D` _returnvalue)))
  (set `self.Location` (- (`KismetMathLibrary.Normal` (`self.Location`)) (`KismetMathLibrary.MakeVector` 0.0 (- 1.0 (`KismetMathLibrary.FClamp` (`KismetMathLibrary.NormalizeToRange` (`self.Mouse X`) 0.0 (* _returnvalue_x_3 0.05))))) (`KismetMathLibrary.MakeVector` 0.0 (* (`KismetMathLibrary.FClamp` (`KismetMathLibrary.NormalizeToRange` (`self.Mouse X`) (* _returnvalue_x_4 0.95) _returnvalue_x_4)) -1.0)) (`KismetMathLibrary.MakeVector` (- 1.0 (`KismetMathLibrary.FClamp` (`KismetMathLibrary.NormalizeToRange` (`self.Mouse Y`) (* 0.05 _returnvalue_y_2))))) (`KismetMathLibrary.MakeVector` (* (`KismetMathLibrary.FClamp` (`KismetMathLibrary.NormalizeToRange` (`self.Mouse Y`) (* 0.95 _returnvalue_y) _returnvalue_y)) -1.0)))))

(fn `UserConstructionScript`)