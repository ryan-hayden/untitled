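; BP_Action_UseAbility is a player action in the combat setup that fires an ability at a chosen tile.
; ExecuteAction passes the action's Ability, the currently selected tile as origin and the given index as target to the combat system's UseAbility.
; It then resets the selected unit's action and movement points, if a unit is selected.
; The event graph holds only disabled default events.
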(fn `ExecuteAction`
  (params (Index :type "IntPoint Structure"))
  (bind _selectedunit (`/Game/Blueprints/Core/Player/BP_PlayerActions.SelectedUnit` (`self.PlayerActions`)))
  (`/Game/Blueprints/Core/Combat/BP_CombatSystem.UseAbility` (`/Game/Blueprints/Core/Player/BP_PlayerActions.CombatSystem` (`self.PlayerActions`)) (`self.Ability`) (`/Game/Blueprints/Core/Player/BP_PlayerActions.SelectedTile` (`self.PlayerActions`)) (`local.Index`))
  (`/Engine/EditorBlueprintResources/StandardMacros.IsValid` _selectedunit
    (:`Is Valid`
      (`/Game/Blueprints/Core/Units/BP_Unit.ResetActionPoints` _selectedunit)
      (`/Game/Blueprints/Core/Units/BP_Unit.ResetMovementPoints` _selectedunit))))

(fn `UserConstructionScript`
  (`parent.UserConstructionScript`))