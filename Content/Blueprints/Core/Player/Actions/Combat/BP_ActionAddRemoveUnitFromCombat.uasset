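; Player action that adds or removes a combat unit on a grid tile, chosen by the IsAddingUnit flag.
; When adding to a walkable tile, it removes and destroys any unit already there, then spawns a BP_Unit of the set UnitType and registers it with the CombatSystem at that index.
; When removing, it reuses the same remove-and-destroy step without the walkability check.
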(fn `ExecuteAction`
  (params (Index :type "IntPoint Structure"))
  (bind (_index _type _transform _states _unitontile) (break `/Game/Blueprints/Core/Grid/Utilities/S_TileData` (`BlueprintMapLibrary.Map_Find` (`/Game/Blueprints/Core/Grid/BP_HexGrid.GridTiles` (`/Game/Blueprints/Core/Player/BP_PlayerActions.Grid` (`self.PlayerActions`))) (`local.Index`))))
  (if (`self.IsAddingUnit`)
    (if (`/Game/Blueprints/Core/Grid/BP_HexGrid.IsTileWalkable` (`/Game/Blueprints/Core/Player/BP_PlayerActions.Grid` (`self.PlayerActions`)) (`local.Index`))
      (`|ExecutionSequence`
        (:`then_0`
          (`/Engine/EditorBlueprintResources/StandardMacros.IsValid` _unitontile :!label _label
            (:`Is Valid`
              (`/Game/Blueprints/Core/Combat/BP_CombatSystem.RemoveUnitFromCombat` (`/Game/Blueprints/Core/Player/BP_PlayerActions.CombatSystem` (`self.PlayerActions`)) _unitontile true))))
        (:`then_1`
          (bind _returnvalue (`|SpawnActorFromClass` "/Game/Blueprints/Core/Units/BP_Unit.BP_Unit_C" (`KismetMathLibrary.MakeTransform` (0.0 0.0 0.0)) "Undefined" "MultiplyWithRoot" null (`self.UnitType`) null))
          (`/Game/Blueprints/Core/Combat/BP_CombatSystem.AddUnitInCombat` (`/Game/Blueprints/Core/Player/BP_PlayerActions.CombatSystem` (`self.PlayerActions`)) _returnvalue (`local.Index`)))))
    (else
      (goto _label))))

(fn `UserConstructionScript`
  (`parent.UserConstructionScript`))