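; Player action for using a combat ability from the selected tile on a clicked grid tile.
; Setting an ability loads its use and AOE data, then marks range tiles through CombatSystem range queries.
; Hovering a tile within range previews the AOE pattern, or just that tile if none.
; Executing calls CombatSystem UseAbility and resets the overlay's ability selection; clearing the ability or EndPlay removes both highlight states.
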(event `self.ReceiveEndPlay`
  (params (EndPlayReason :type "EEndPlayReason Enum" :default "Destroyed"))
  (bind _grid (`/Game/Blueprints/Core/Player/BP_PlayerActions.Grid` (`self.PlayerActions`)))
  (`parent.ReceiveEndPlay` EndPlayReason)
  (`/Game/Blueprints/Core/Grid/BP_HexGrid.ClearStateFromTiles` _grid "NewEnumerator8")
  (`/Game/Blueprints/Core/Grid/BP_HexGrid.ClearStateFromTiles` _grid "NewEnumerator9"))

(fn `ExecuteAction`
  (params (Index :type "IntPoint Structure"))
  (bind _playeractions (`self.PlayerActions`))
  (bind _w_mainoverlay (`/Game/Blueprints/Core/Player/BP_PlayerActions.W_MainOverlay` (`self.PlayerActions`)))
  (`parent.ExecuteAction` Index)
  (`/Game/Blueprints/Core/Combat/BP_CombatSystem.UseAbility` (`/Game/Blueprints/Core/Player/BP_PlayerActions.CombatSystem` _playeractions) (`self.Ability`) (`/Game/Blueprints/Core/Player/BP_PlayerActions.SelectedTile` _playeractions) (`local.Index`))
  (`/Engine/EditorBlueprintResources/StandardMacros.IsValid` _w_mainoverlay ; widget is destroyed during the finishing game phase
    (:`Is Valid`
      (`/Game/Blueprints/Core/Combat/Abilities/Widget/ButtonList_Abilities.SetSelectedAbilityFromIndex` (`/Game/Blueprints/Core/UI/Widgets/W_MainOverlayUI.ButtonList_Abilities` _w_mainoverlay) -1))))

(fn `ExecuteHoveredAction`
  (params (Index :type "IntPoint Structure"))
  (`parent.ExecuteHoveredAction` Index)
  (`self.ShowAbilityRangeAoePattern`))

(fn `SetAbility`
  (params (Ability :type "/Game/Blueprints/Core/Combat/Abilities/Utilities/E_Ability Enum" :default "NewEnumerator0"))
  (bind _grid (`/Game/Blueprints/Core/Player/BP_PlayerActions.Grid` (`self.PlayerActions`)))
  (bind _output_get (set `self.Ability` Ability))
  (if (`|EnumInequality` _output_get "NewEnumerator0")
    (bind _ability_data (`/Game/Blueprints/Core/Combat/Abilities/Utilities/BFL_Abilities.GetAbilityDataFromAbility` (`self.Ability`)))
    (bind (_ability _assets _use _abilityaoe) (break `/Game/Blueprints/Core/Combat/Abilities/Utilities/S_AbilityData` _ability_data))
    (set `self.UseData` _use)
    (set `self.Ability AOE` _abilityaoe)
    (`self.ShowAbilityRangePattern`)
    (else
      (`/Game/Blueprints/Core/Grid/BP_HexGrid.ClearStateFromTiles` _grid "NewEnumerator8")
      (`/Game/Blueprints/Core/Grid/BP_HexGrid.ClearStateFromTiles` _grid "NewEnumerator9"))))

(fn `ShowAbilityRangeAoePattern`
  (bind _playeractions (`self.PlayerActions`))
  (bind _playeractions_2 (`self.PlayerActions`))
  (`/Game/Blueprints/Core/Grid/BP_HexGrid.ClearStateFromTiles` (`/Game/Blueprints/Core/Player/BP_PlayerActions.Grid` (`self.PlayerActions`)) "NewEnumerator9")
  (if (`KismetArrayLibrary.Array_Contains` (`.IntPointArray_3_589AE0FB4365210FBA4173A321F13988` (break `/Game/Blueprints/Core/Grid/Utilities/S_IntPointArray` (`BlueprintMapLibrary.Map_Find` (`/Game/Blueprints/Core/Grid/BP_HexGrid.TileStateToIndexes` (`/Game/Blueprints/Core/Player/BP_PlayerActions.Grid` (`self.PlayerActions`))) "NewEnumerator8"))) (`/Game/Blueprints/Core/Player/BP_PlayerActions.HoveredTile` (`self.PlayerActions`)))
    (if (`|EnumInequality` (`.RangePattern_5_1A81E52D4876460BDA20048B3425F955` (break `/Game/Blueprints/Core/Combat/Abilities/Utilities/S_AbilityData_Use` (`self.Ability AOE`))) "NewEnumerator0")
      (bind _rangeindexes (`/Game/Blueprints/Core/Combat/BP_CombatSystem.GetAbilityRange` (`/Game/Blueprints/Core/Player/BP_PlayerActions.CombatSystem` _playeractions_2) (`/Game/Blueprints/Core/Player/BP_PlayerActions.HoveredTile` _playeractions_2) (`self.Ability AOE`)))
      (for _array_element _rangeindexes
        (`/Game/Blueprints/Core/Grid/BP_HexGrid.AddStateToTile` (`/Game/Blueprints/Core/Player/BP_PlayerActions.Grid` (`self.PlayerActions`)) _array_element "NewEnumerator9"))
      (else
        (`/Game/Blueprints/Core/Grid/BP_HexGrid.AddStateToTile` (`/Game/Blueprints/Core/Player/BP_PlayerActions.Grid` _playeractions) (`/Game/Blueprints/Core/Player/BP_PlayerActions.HoveredTile` _playeractions) "NewEnumerator9")))))

(fn `ShowAbilityRangePattern`
  (bind _playeractions (`self.PlayerActions`))
  (`|ExecutionSequence`
    (:`then_0`
      (`/Game/Blueprints/Core/Grid/BP_HexGrid.ClearStateFromTiles` (`/Game/Blueprints/Core/Player/BP_PlayerActions.Grid` (`self.PlayerActions`)) "NewEnumerator8")
      (bind _rangeindexes (`/Game/Blueprints/Core/Combat/BP_CombatSystem.GetAbilityRange` (`/Game/Blueprints/Core/Player/BP_PlayerActions.CombatSystem` _playeractions) (`/Game/Blueprints/Core/Player/BP_PlayerActions.SelectedTile` _playeractions) (`self.UseData`)))
      (for _array_element _rangeindexes
        (`/Game/Blueprints/Core/Grid/BP_HexGrid.AddStateToTile` (`/Game/Blueprints/Core/Player/BP_PlayerActions.Grid` (`self.PlayerActions`)) _array_element "NewEnumerator8")))
    (:`then_1`
      (`self.ShowAbilityRangeAoePattern`))))

(fn `UserConstructionScript`
  (`parent.UserConstructionScript`))