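; Ability animation actor for the Dark Wave combat ability, shown as a purple-blue wave effect at the target tile.
; On play, it moves to the target tile, and a timeline drives the effect's scale and the opacity of three tinted meshes.
; Shortly into the timeline, a DoOnce reports a hit on every attacked tile at once.
; The animation signals completion when the timeline finishes.
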(event `self.Event_PlayAbilityAnimation`
  (bind _transform_location (`KismetMathLibrary.BreakTransform` (`self.GetTileTransform` (`self.TargetIndex`))))
  (`self.K2_SetActorLocation` _transform_location)
  (bind (_direction _opacity _scale) (`Timeline|Timeline_DarkWave`)
    (:`Update`
      (`SceneComponent.SetRelativeScale3D` (`self.Anim Scale`) _scale)
      (`MeshComponent.SetScalarParameterValueOnMaterials` (`self.StaticMesh`) "Opacity" _opacity)
      (`MeshComponent.SetScalarParameterValueOnMaterials` (`self.StaticMesh2`) "Opacity" _opacity)
      (`MeshComponent.SetScalarParameterValueOnMaterials` (`self.StaticMesh1`) "Opacity" _opacity)
      (if (>= (`TimelineComponent.GetPlaybackPosition` (`self.Timeline_DarkWave`)) 0.2)
        (`/Engine/EditorBlueprintResources/StandardMacros.DoOnce` false
          (:`Completed`
            (for _array_element (`self.AttackedIndexes`)
              (`self.OnAbilityAnimationHitTile` self _array_element))))))
    (:`Finished`
      (`self.Event Complete Ability Animation Completed`))))

(fn `UserConstructionScript`
  (`parent.UserConstructionScript`)
  (`MeshComponent.SetVectorParameterValueOnMaterials` (`self.StaticMesh`) "LaserColor" (`KismetMathLibrary.Conv_LinearColorToVector` (struct :`R` 0.434498 :`B` 0.71875 :`A` 1.0)))
  (`MeshComponent.SetVectorParameterValueOnMaterials` (`self.StaticMesh1`) "LaserColor" (`KismetMathLibrary.Conv_LinearColorToVector` (struct :`R` 0.272367 :`B` 0.71875 :`A` 1.0)))
  (`MeshComponent.SetVectorParameterValueOnMaterials` (`self.StaticMesh2`) "LaserColor" (`KismetMathLibrary.Conv_LinearColorToVector` (struct :`R` 0.099957 :`B` 1.0 :`A` 1.0))))