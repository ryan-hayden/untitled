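; BP_AbilityAnim_ExplodeArrow is an ability animation that shoots an arrow between two grid tiles and ends in an explosion.
; It faces the target tile, then a timeline drives position, height offset, pitch and scale along the flight.
; A DoOnce reports the tile hit once playback passes a set point.
; On arrival the arrow mesh hides and a second timeline scales the explosion and animates its opacity before signaling completion.
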(event `self.Event_PlayAbilityAnimation`
  (bind _explosionmesh (`self.ExplosionMesh`))
  (bind _transform_location (`KismetMathLibrary.BreakTransform` (`self.GetTileTransform` (`self.StartingIndex`))))
  (bind _transform_location_2 (`KismetMathLibrary.BreakTransform` (`self.GetTileTransform` (`self.StartingIndex`))))
  (bind _transform_location_3 (`KismetMathLibrary.BreakTransform` (`self.GetTileTransform` (`self.TargetIndex`))))
  (`SceneComponent.SetVisibility` (`self.ExplosionMesh`) false false)
  (`self.K2_SetActorLocationAndRotation` _transform_location_2 (`KismetMathLibrary.FindLookAtRotation` (`KismetMathLibrary.Conv_Vector2DToVector` (`KismetMathLibrary.Conv_IntPointToVector2D` (`self.StartingIndex`))) (`KismetMathLibrary.Conv_Vector2DToVector` (`KismetMathLibrary.Conv_IntPointToVector2D` (`self.TargetIndex`)))))
  (bind (_direction _location_alpha _location_z _rotation_y _scale) (`Timeline|Timeline_ShootArrow`)
    (:`Update`
      (`self.K2_SetActorLocation` (+ (`KismetMathLibrary.VLerp` _transform_location _transform_location_3 _location_alpha) (`KismetMathLibrary.MakeVector` 0.0 0.0 _location_z)))
      (`SceneComponent.K2_SetRelativeTransform` (`self.Anim_LocationAndRotation`) (`KismetMathLibrary.MakeTransform` (0.0 0.0 0.0) (`KismetMathLibrary.MakeRotator` 0.0 _rotation_y) (`KismetMathLibrary.Conv_DoubleToVector` _scale)) false false)
      (if (>= (`TimelineComponent.GetPlaybackPosition` (`self.Timeline_ShootArrow`)) 0.69)
        (`/Engine/EditorBlueprintResources/StandardMacros.DoOnce` false
          (:`Completed`
            (`self.OnAbilityAnimationHitTile` self (`self.TargetIndex`))))))
    (:`Finished`
      (`SceneComponent.SetVisibility` (`self.StaticMesh`) false false)
      (`SceneComponent.SetVisibility` (`self.ExplosionMesh`) true false)
      (bind (_direction_2 _scale_2 _opacity) (`Timeline|Timeline_Explosion`)
        (:`Update`
          (`SceneComponent.SetRelativeScale3D` _explosionmesh (`KismetMathLibrary.Conv_DoubleToVector` _scale_2))
          (`MeshComponent.SetScalarParameterValueOnMaterials` _explosionmesh "Opacity" _opacity))
        (:`Finished`
          (`self.Event Complete Ability Animation Completed`))))))

(fn `UserConstructionScript`
  (`parent.UserConstructionScript`))