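; Ability animation actor that shows a visual cue for a movement buff on a target tile.
; When played, it moves to the target tile and sets its widget's image to the RunChickenRun icon.
; A timeline drives the widget's height, draw size and opacity, then signals that the ability animation is complete.
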(event `self.Event_PlayAbilityAnimation`
  (bind _widget (`self.Widget`))
  (bind _transform_location (`KismetMathLibrary.BreakTransform` (`self.GetTileTransform` (`self.TargetIndex`))))
  (`self.K2_SetActorLocation` _transform_location)
  (bind _output_get (set `self.W Image` (cast `/Game/Blueprints/Core/Combat/Abilities/AbilityAnimations/Components/W_Image` (`WidgetComponent.GetUserWidgetObject` (`self.Widget`)) :!pure true)))
  (`Image.SetBrushFromTexture` (`/Game/Blueprints/Core/Combat/Abilities/AbilityAnimations/Components/W_Image.Image_Component` _output_get) "/Game/Blueprints/Core/Combat/Abilities/AbilityAnimations/Assets/Icon_RunChickenRun_NoBackground.Icon_RunChickenRun_NoBackground" false)
  (bind (_direction _location_z _draw_size _opacity) (`Timeline|Timeline_MovementBuff`)
    (:`Update`
      (`SceneComponent.K2_SetRelativeLocation` _widget (`KismetMathLibrary.MakeVector` 0.0 0.0 _location_z) false false)
      (`WidgetComponent.SetDrawSize` _widget (`KismetMathLibrary.MakeVector2D` _draw_size _draw_size))
      (`Widget.SetRenderOpacity` (`self.W Image`) _opacity))
    (:`Finished`
      (`self.Event Complete Ability Animation Completed`))))

(fn `UserConstructionScript`
  (`parent.UserConstructionScript`))