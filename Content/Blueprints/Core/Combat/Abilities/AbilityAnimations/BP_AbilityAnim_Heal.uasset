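; Ability animation actor that plays the heal visual effect on a target tile.
; The construction script tints three meshes and three health particle components in shades of green.
; When played, it moves to the target tile and runs a timeline that rotates and scales the AnimScale component and drives material opacity.
; It signals animation completion when the timeline finishes.
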(event `self.Event_PlayAbilityAnimation`
  (bind _transform_location (`KismetMathLibrary.BreakTransform` (`self.GetTileTransform` (`self.TargetIndex`))))
  (`self.K2_SetActorLocation` _transform_location)
  (bind (_direction _opacity _scale _rotation_z) (`Timeline|Timeline`)
    (:`Update`
      (`SceneComponent.K2_SetRelativeRotation` (`self.Anim Scale`) (`KismetMathLibrary.MakeRotator` 0.0 0.0 _rotation_z) false false)
      (`SceneComponent.SetRelativeScale3D` (`self.Anim Scale`) _scale)
      (`MeshComponent.SetScalarParameterValueOnMaterials` (`self.StaticMesh`) "Opacity" _opacity)
      (`MeshComponent.SetScalarParameterValueOnMaterials` (`self.StaticMesh2`) "Opacity" _opacity)
      (`MeshComponent.SetScalarParameterValueOnMaterials` (`self.StaticMesh1`) "Opacity" _opacity)
      (`MeshComponent.SetScalarParameterValueOnMaterials` (`self.HealthParticle`) "Opacity" _opacity)
      (`MeshComponent.SetScalarParameterValueOnMaterials` (`self.HealthParticle1`) "Opacity" _opacity)
      (`MeshComponent.SetScalarParameterValueOnMaterials` (`self.HealthParticle2`) "Opacity" _opacity))
    (:`Finished`
      (`self.Event Complete Ability Animation Completed`))))

(fn `UserConstructionScript`
  (`parent.UserConstructionScript`)
  (`MeshComponent.SetVectorParameterValueOnMaterials` (`self.StaticMesh`) "LaserColor" (`KismetMathLibrary.Conv_LinearColorToVector` (struct :`R` 0.182976 :`G` 0.71875 :`A` 1.0)))
  (`MeshComponent.SetVectorParameterValueOnMaterials` (`self.StaticMesh1`) "LaserColor" (`KismetMathLibrary.Conv_LinearColorToVector` (struct :`G` 0.71875 :`B` 0.019972 :`A` 1.0)))
  (`MeshComponent.SetVectorParameterValueOnMaterials` (`self.StaticMesh2`) "LaserColor" (`KismetMathLibrary.Conv_LinearColorToVector` (struct :`G` 1.0 :`B` 0.438498 :`A` 1.0)))
  (`MeshComponent.SetVectorParameterValueOnMaterials` (`self.HealthParticle`) "LaserColor" (`KismetMathLibrary.Conv_LinearColorToVector` (struct :`R` 0.182976 :`G` 0.71875 :`A` 1.0)))
  (`MeshComponent.SetVectorParameterValueOnMaterials` (`self.HealthParticle1`) "LaserColor" (`KismetMathLibrary.Conv_LinearColorToVector` (struct :`G` 0.71875 :`B` 0.019972 :`A` 1.0)))
  (`MeshComponent.SetVectorParameterValueOnMaterials` (`self.HealthParticle2`) "LaserColor" (`KismetMathLibrary.Conv_LinearColorToVector` (struct :`G` 1.0 :`B` 0.438498 :`A` 1.0))))