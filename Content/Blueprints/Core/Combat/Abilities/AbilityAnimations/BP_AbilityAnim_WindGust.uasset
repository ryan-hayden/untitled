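; Ability animation for Wind Gust that fans gusts out from the target tile to the other attacked tiles.
; After a brief delay it reports the target tile as hit, then spawns a BP_AnimatedWindGust toward each remaining tile, scaling up at a randomized play rate.
; Each finished gust reports its tile as hit and is removed from AttackedIndexes, and the last one completes the animation.
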(event `self.Event_PlayAbilityAnimation`
  (bind _targetindex (`self.TargetIndex`))
  (bind _transform_location (`KismetMathLibrary.BreakTransform` (`self.GetTileTransform` (`self.TargetIndex`))))
  (`KismetSystemLibrary.Delay` 0.05)
  (`self.OnAbilityAnimationHitTile` self _targetindex)
  (`KismetArrayLibrary.Array_RemoveItem` (`self.AttackedIndexes`) _targetindex)
  (for _array_element (`self.AttackedIndexes`)
    (bind _transform_location_2 (`KismetMathLibrary.BreakTransform` (`self.GetTileTransform` _array_element)))
    (bind _returnvalue (`KismetMathLibrary.FindLookAtRotation` _transform_location _transform_location_2))
    (bind _returnvalue_2 (`|SpawnActorFromClass` "/Game/Blueprints/Core/Combat/Abilities/AbilityAnimations/Components/BP_AnimatedWindGust.BP_AnimatedWindGust_C" (`KismetMathLibrary.MakeTransform` (0.0 0.0 0.0)) "AlwaysSpawn" "MultiplyWithRoot" null (`KismetMathLibrary.MakeTransform` _transform_location _returnvalue (0.5 1.0 0.5)) (`KismetMathLibrary.MakeTransform` _transform_location_2 _returnvalue (1.2 1.2 1.2)) (`KismetMathLibrary.RandomFloatInRange` 0.8 1.1) _array_element null))
    (add `/Game/Blueprints/Core/Combat/Abilities/AbilityAnimations/Components/BP_AnimatedWindGust.OnShapeAnimationCompleted` _returnvalue_2 (delegate `OnShapeAnimComplete`))))

(event `OnShapeAnimComplete`
  (params (`Wind Gust` :type "/Game/Blueprints/Core/Combat/Abilities/AbilityAnimations/Components/BP_AnimatedWindGust Object Reference"))
  (bind _index (`/Game/Blueprints/Core/Combat/Abilities/AbilityAnimations/Components/BP_AnimatedWindGust.Index` `Wind Gust`))
  (bind _attackedindexes (`self.AttackedIndexes`))
  (`self.OnAbilityAnimationHitTile` self _index)
  (`KismetArrayLibrary.Array_RemoveItem` _attackedindexes _index)
  (if (== (`KismetArrayLibrary.Array_Length` _attackedindexes) 0)
    (`self.Event Complete Ability Animation Completed`)))

(fn `UserConstructionScript`
  (`parent.UserConstructionScript`))