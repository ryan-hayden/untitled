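; Short-lived wind gust visual actor for a combat ability animation, which moves itself from an origin to a target transform.
; Construction gives its two material slots translucent dynamic instances in green shades with randomized brightness.
; On BeginPlay a rate-adjustable timeline drives the transform lerp and material opacity.
; It signals shape-animation completion once partway through playback, before the timeline ends, then destroys itself shortly after the timeline finishes.
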(event `self.ReceiveBeginPlay`
  (`TimelineComponent.SetPlayRate` (`self.Timeline_PlayAnimation`) (`self.Play Rate`))
  (bind (_direction _transform_alpha _opacity) (`Timeline|Timeline_PlayAnimation` :!via `PlayFromStart`)
    (:`Update`
      (`self.K2_SetActorTransform` (`KismetMathLibrary.TLerp` (`self.Origin Transform`) (`self.Target Transform`) _transform_alpha))
      (`MeshComponent.SetScalarParameterValueOnMaterials` (`self.AnimatedWindGust`) "Opacity" _opacity)
      (if (>= (`TimelineComponent.GetPlaybackPosition` (`self.Timeline_PlayAnimation`)) 0.3)
        (`/Engine/EditorBlueprintResources/StandardMacros.DoOnce` false
          (:`Completed`
            (`self.OnShapeAnimationCompleted` self)))))
    (:`Finished`
      (`KismetSystemLibrary.Delay` 0.5)
      (`self.K2_DestroyActor`))))

(fn `UserConstructionScript`
  (bind _returnvalue (`PrimitiveComponent.CreateDynamicMaterialInstance` (`self.AnimatedWindGust`) 0 "/Engine/VREditor/LaserPointer/TranslucentLaserPointerMaterialInst.TranslucentLaserPointerMaterialInst" "None"))
  (`MaterialInstanceDynamic.SetVectorParameterValue` _returnvalue "LaserColor" (* (struct :`G` 1.0 :`B` 0.187191 :`A` 1.0) (`KismetMathLibrary.RandomFloatInRange` 0.8 1.5)))
  (bind _returnvalue_2 (`PrimitiveComponent.CreateDynamicMaterialInstance` (`self.AnimatedWindGust`) 1 "/Engine/VREditor/LaserPointer/TranslucentLaserPointerMaterialInst.TranslucentLaserPointerMaterialInst" "None"))
  (`MaterialInstanceDynamic.SetVectorParameterValue` _returnvalue_2 "LaserColor" (* (struct :`R` 0.441778 :`G` 0.807292 :`A` 1.0) (`KismetMathLibrary.RandomFloatInRange` 0.8 1.5))))