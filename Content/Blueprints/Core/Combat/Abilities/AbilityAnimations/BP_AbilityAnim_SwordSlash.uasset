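; Ability animation actor that plays a sword slash from a starting grid tile toward a target tile.
; When played, it moves to the starting tile and faces the target using the look-at rotation between the two tile indices.
; A timeline drives the pitch and scale of its animated component, signals a hit on the target tile once near a fixed playback time, then reports completion when finished.
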(event `self.Event_PlayAbilityAnimation`
  (bind _anim_rotationandscale (`self.Anim_RotationAndScale`))
  (bind _transform_location (`KismetMathLibrary.BreakTransform` (`self.GetTileTransform` (`self.StartingIndex`))))
  (`self.K2_SetActorLocationAndRotation` _transform_location (`KismetMathLibrary.FindLookAtRotation` (`KismetMathLibrary.Conv_Vector2DToVector` (`KismetMathLibrary.Conv_IntPointToVector2D` (`self.StartingIndex`))) (`KismetMathLibrary.Conv_Vector2DToVector` (`KismetMathLibrary.Conv_IntPointToVector2D` (`self.TargetIndex`)))))
  (bind (_direction _rotation_y _scale) (`Timeline|Timeline_SwordSlash`)
    (:`Update`
      (`SceneComponent.K2_SetRelativeRotation` _anim_rotationandscale (`KismetMathLibrary.MakeRotator` 0.0 _rotation_y) false false)
      (`SceneComponent.SetRelativeScale3D` _anim_rotationandscale (`KismetMathLibrary.Conv_DoubleToVector` _scale))
      (if (>= (`TimelineComponent.GetPlaybackPosition` (`self.Timeline_SwordSlash`)) 0.91)
        (`/Engine/EditorBlueprintResources/StandardMacros.DoOnce` false
          (:`Completed`
            (`self.OnAbilityAnimationHitTile` self (`self.TargetIndex`))))))
    (:`Finished`
      (`self.Event Complete Ability Animation Completed`))))

(fn `UserConstructionScript`
  (`parent.UserConstructionScript`))