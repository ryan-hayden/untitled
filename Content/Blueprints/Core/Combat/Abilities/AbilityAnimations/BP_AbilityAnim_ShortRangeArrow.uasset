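; Ability animation actor for a short-range arrow, flying from a starting tile to a target tile in grid combat.
; On play, it snaps to the start tile, rotates toward the target using grid indices, and runs Timeline_SwordThrow.
; The timeline lerps position with an added world-Y offset from its LocationZ track, while pitching and scaling the AnimLocationAndRotation component.
; When the timeline finishes, it signals ability animation completion.
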(event `self.Event_PlayAbilityAnimation`
  (bind _transform_location (`KismetMathLibrary.BreakTransform` (`self.GetTileTransform` (`self.StartingIndex`))))
  (bind _transform_location_2 (`KismetMathLibrary.BreakTransform` (`self.GetTileTransform` (`self.StartingIndex`))))
  (bind _transform_location_3 (`KismetMathLibrary.BreakTransform` (`self.GetTileTransform` (`self.TargetIndex`))))
  (`self.K2_SetActorLocationAndRotation` _transform_location_2 (`KismetMathLibrary.FindLookAtRotation` (`KismetMathLibrary.Conv_Vector2DToVector` (`KismetMathLibrary.Conv_IntPointToVector2D` (`self.StartingIndex`))) (`KismetMathLibrary.Conv_Vector2DToVector` (`KismetMathLibrary.Conv_IntPointToVector2D` (`self.TargetIndex`)))))
  (bind (_direction _location_alpha _location_z _rotation_y _scale) (`Timeline|Timeline_SwordThrow`)
    (:`Update`
      (`self.K2_SetActorLocation` (+ (`KismetMathLibrary.VLerp` _transform_location _transform_location_3 _location_alpha) (`KismetMathLibrary.MakeVector` 0.0 _location_z)))
      (`SceneComponent.K2_SetRelativeTransform` (`self.Anim_LocationAndRotation`) (`KismetMathLibrary.MakeTransform` (0.0 0.0 0.0) (`KismetMathLibrary.MakeRotator` 0.0 _rotation_y) (`KismetMathLibrary.Conv_DoubleToVector` _scale)) false false))
    (:`Finished`
      (`self.Event Complete Ability Animation Completed`))))

(fn `UserConstructionScript`
  (`parent.UserConstructionScript`))