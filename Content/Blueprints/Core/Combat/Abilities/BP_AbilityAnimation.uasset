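; Short-lived actor that animates a combat ability on the grid from a starting tile to each attacked tile.
; On BeginPlay it spawns one BP_AnimatedShape per attacked index, using the grid's current shape mesh and material with randomized tint brightness and play rate.
; Each finished shape broadcasts a tile-hit event and removes its index; when none remain, the actor broadcasts completion and destroys itself.
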(event `self.ReceiveBeginPlay`
  (`self.Event_PlayAbilityAnimation`))

(event `Event_PlayAbilityAnimation`
  (bind _returnvalue (`KismetMathLibrary.RandomFloatInRange` 0.5 1.5))
  (bind (_transform_location _transform_rotation) (`KismetMathLibrary.BreakTransform` (`self.GetTileTransform` (`self.StartingIndex`))))
  (bind (_meshsize _mesh _meshmaterial) (break `/Game/Blueprints/Core/Grid/S_GridShapeData` (`/Game/Blueprints/Core/Grid/BP_HexGrid.GetCurrentShapeData` (`self.Grid`))))
  (for _array_element (`self.AttackedIndexes`)
    (bind _returnvalue_2 (`|SpawnActorFromClass` "/Game/Blueprints/Core/Combat/Abilities/AbilityAnimations/Components/BP_AnimatedShape.BP_AnimatedShape_C" (`KismetMathLibrary.MakeTransform` (0.0 0.0 0.0)) "AlwaysSpawn" "MultiplyWithRoot" null _mesh _meshmaterial (* _returnvalue (struct :`R` 0.00675 :`G` 0.840088 :`B` 1.0 :`A` 1.0)) (`KismetMathLibrary.MakeTransform` _transform_location _transform_rotation (0.1 0.1 0.1)) (`self.GetTileTransform` _array_element) _returnvalue _array_element null))
    (add `/Game/Blueprints/Core/Combat/Abilities/AbilityAnimations/Components/BP_AnimatedShape.OnShapeAnimationCompleted` _returnvalue_2 (delegate `OnShapeAnimationCompleted`))))

(event `OnShapeAnimationCompleted`
  (params (AnimatedShape :type "/Game/Blueprints/Core/Combat/Abilities/AbilityAnimations/Components/BP_AnimatedShape Object Reference"))
  (bind _index (`/Game/Blueprints/Core/Combat/Abilities/AbilityAnimations/Components/BP_AnimatedShape.Index` AnimatedShape))
  (bind _attackedindexes (`self.AttackedIndexes`))
  (`self.OnAbilityAnimationHitTile` self _index)
  (`KismetArrayLibrary.Array_RemoveItem` _attackedindexes _index)
  (if (== (`KismetArrayLibrary.Array_Length` _attackedindexes) 0)
    (`self.Event Complete Ability Animation Completed`)))

(event `Event Complete Ability Animation Completed`
  (`self.OnAbilityAnimationCompleted` null)
  (`self.K2_DestroyActor`))

(fn `GetTileTransform`
  (params (Index :type "IntPoint Structure (by ref)"))
  (returns (Transform :type "Transform Structure"))
  (return (`.Transform_8_1D847D9A429058A71E48E482CDEF505D` (break `/Game/Blueprints/Core/Grid/Utilities/S_TileData` (`BlueprintMapLibrary.Map_Find` (`/Game/Blueprints/Core/Grid/BP_HexGrid.GridTiles` (`self.Grid`)) Index)))))

(fn `UserConstructionScript`)